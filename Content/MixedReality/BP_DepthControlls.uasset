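; Debug keyboard control Blueprint for toggling mixed reality depth features at runtime.
; On BeginPlay it enables input from the first player controller.
; The T, E and R keys flip depth testing, environment depth estimation and the depth test range, each by inverting its current state.
; The range toggle preserves the existing near and far Z limits.
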(event `self.ReceiveBeginPlay`
  (`self.EnableInput` (`GameplayStatics.GetPlayerController` 0)))

(event `Key|T`
  (params (Key :type "Key Structure"))
  ;[1 1 1] Toggle Depth Testing
  (:`Pressed`
    (`VarjoOpenXRFunctionLibrary.SetDepthTestEnabled` (not (`VarjoOpenXRFunctionLibrary.IsDepthTestEnabled`)))))

(event `Key|E`
  (params (Key :type "Key Structure"))
  ;[1 1 1] Toggle Environment Depth Estimation
  (:`Pressed`
    (`VarjoOpenXRFunctionLibrary.SetEnvironmentDepthEstimationEnabled` (not (`VarjoOpenXRFunctionLibrary.IsEnvironmentDepthEstimationEnabled`)))))

(event `Key|R`
  (params (Key :type "Key Structure"))
  (bind (_bisenabled _nearz _farz) (`VarjoOpenXRFunctionLibrary.GetDepthTestRange`))
  ;[1 1 1] Toggle Depth Test Range
  (:`Pressed`
    (`VarjoOpenXRFunctionLibrary.SetDepthTestRange` (not _bisenabled) _nearz _farz)))

(fn `UserConstructionScript`)