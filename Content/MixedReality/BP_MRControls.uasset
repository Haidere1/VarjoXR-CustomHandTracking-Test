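; BP_MRControls is an input actor that switches the headset between opaque VR and mixed reality.
; The MRToggle action checks mixed reality support, then flips the environment blend mode between Opaque and Alpha Blend.
; The B key separately flips a background flag that hides or shows the listed VR-only objects and their child components.
; On BeginPlay it enables player input and caches the HandTracking actor as VRPawn.
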(event `self.ReceiveBeginPlay`
  (`self.EnableInput` (`GameplayStatics.GetPlayerController` 0))
  (bind _returnvalue (`GameplayStatics.GetActorOfClass` "/Script/VarjoXRGAME.HandTracking"))
  (set `self.VRPawn` _returnvalue))

(event `InputAction|MRToggle`
  (params (Key :type "Key Structure"))
  ;[1 1 1] Toggle Mixed Reality rendering
  (:`Pressed`
    (if (`VarjoOpenXRFunctionLibrary.IsMixedRealitySupported`)
      (if (`VarjoOpenXRFunctionLibrary.IsMixedRealityEnabled`)
        (`OpenXRBlueprintFunctionLibrary.SetEnvironmentBlendMode` 1) ; Opaque
        (else
          (`OpenXRBlueprintFunctionLibrary.SetEnvironmentBlendMode` 3) ; Alpha Blend
        )))))

(event `Key|B`
  (params (Key :type "Key Structure"))
  ;[1 1 1] Toggle Mixed Reality Background
  (:`Pressed`
    (bind _output_get (set `self.MRBackground` (not (`self.MRBackground`))))
    (for _array_element (`self.VROnlyObjects`)
      (`SceneComponent.SetVisibility` (`Actor.RootComponent` _array_element) (not _output_get) true))))

(fn `UserConstructionScript`)